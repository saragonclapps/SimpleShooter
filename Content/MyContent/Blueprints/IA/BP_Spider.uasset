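; Spider enemy character that chases and attacks the player.
; A retrying AI MoveTo loop targets the player, while Tick enables movement only when the player is inside the CollisionActive zone.
; Within attack range, it stops and plays an attack montage; DamagePlayer applies the hit but is not called within this Blueprint.
; Incoming damage lowers health, and at zero it disables movement and collision, then destroys itself after a delay.
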(event OnComponentBeginOverlap(CollisionActive)
  (params (OverlappedComponent :type Primitive%20Component%20Object%20Reference) (OtherActor :type Actor%20Object%20Reference) (OtherComp :type Primitive%20Component%20Object%20Reference) (OtherBodyIndex :type Integer) (bFromSweep :type Boolean) (SweepResult :type Hit%20Result%20Structure%20%28by%20ref%29))
  (if (== OtherActor (Game|Player|GetPlayerPawn 0))
    (Variables|Default|SetIsInZone true)))

(event OnComponentEndOverlap(CollisionActive)
  (params (OverlappedComponent :type Primitive%20Component%20Object%20Reference) (OtherActor :type Actor%20Object%20Reference) (OtherComp :type Primitive%20Component%20Object%20Reference) (OtherBodyIndex :type Integer))
  (if (== OtherActor (Game|Player|GetPlayerPawn 0))
    (Variables|Default|SetIsInZone false)))

(event EventBeginPlay
  (IA|ActivateIAMovement)
  (if (CallFunction|IsAlive) :!label _label
    (AI|AIMoveTo self "0, 0, 0" (Game|GetPlayerCharacter 0) 5.0 false
      (:OnSuccess
        _)
      (:OnFail
        _))
    (Utilities|FlowControl|Delay 0.2)
    (goto _label)))

(event Game|Damage|EventAnyDamage
  (params (Damage :type Float%20%28single-precision%29) (DamageType :type Damage%20Type%20Object%20Reference) (InstigatedBy :type Controller%20Object%20Reference) (DamageCauser :type Actor%20Object%20Reference))
  (if (CallFunction|IsAlive)
    (bind _health (CallFunction|DecreaseHealth Damage))
    (if (<= _health 0.0)
      (IA|KillIA)
      (Utilities|FlowControl|Delay 3.0)
      (Actor|DestroyActor))))

(event EventTick
  (params (DeltaSeconds :type Float%20%28single-precision%29))
  (if (Variables|Default|GetIsInZone)
    (IA|ActivateIAMovement)
    (if (CallFunction|CanAttack)
      (IA|DesactivateIAMovement)
      (Animation|Montage|PlayMontage (Variables|Character|GetMesh) "/Game/MyContent/Characters/Enemy_Great_Spider/Animations/SpiderAttack_AnimMontage.SpiderAttack_AnimMontage"
        (:OnCompleted
          (IA|ActivateIAMovement))))
    (else
      (IA|DesactivateIAMovement))))

(fn ConstructionScript)

(fn IsAlive
  (return (not (Variables|Default|GetDead))))

(fn IsAttacking
  (return (Animation|Montage|MontageIsPlaying (Components|SkeletalMesh|GetAnimInstance (Variables|Character|GetMesh)) 0)))

(fn CanAttack
  (return (Math|Boolean|ANDBoolean (CallFunction|IsWithinAttackRange) (not (CallFunction|IsAttacking)) (CallFunction|IsAlive))))

(fn IsWithinAttackRange
  (return (< (Transformation|GetDistanceTo (Game|Player|GetPlayerPawn 0)) (Variables|Default|GetAttack%20Range))))

(fn DesactivateIAMovement
  (bind _charactermovement (Variables|Character|GetCharacterMovement))
  (Components|Movement|StopMovementImmediately _charactermovement)
  (Components|Activation|Deactivate _charactermovement)
  (return))

(fn DecreaseHealth
  (params (Damage :type Float%20%28single-precision%29))
  (bind _output_get (Variables|Default|SetHealth (Math|Float|Clamp(Float) (- (Variables|Default|GetHealth) Damage) 0.0 1e+02)))
  (return _output_get))

(fn KillIA
  (Variables|Default|SetDead true)
  (IA|DesactivateIAMovement)
  (Collision|SetActorEnableCollision false))

(fn DamagePlayer
  (if (CallFunction|IsAlive)
    (bind _asshooter_character (Utilities|Casting|CastToShooterCharacter (Game|GetPlayerCharacter 0)))
    (Game|Damage|ApplyDamage _asshooter_character (Variables|Default|GetDamage%20per%20Hit) 0 0)))

(fn ActivateIAMovement
  (Components|Activation|Activate (Variables|Character|GetCharacterMovement) false)
  (return))