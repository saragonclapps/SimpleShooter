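; Game mode that ends the game with a win once every non-player shooter character and spider is destroyed.
; On BeginPlay it binds one destroy handler to all existing BP_ShooterCharacter and BP_Spider actors.
; When a non-player dies, the handler recounts both classes, discounting the player and the dying actor, and calls EndGame when none remain.
; Player destruction triggers nothing on the path shown here.
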(event Custom|EventDestroy
  (params (DestroyedActor :type Actor%20Object%20Reference))
  (Utilities|IsPlayer DestroyedActor
    (:NotPlayer
      (bind _outactors (Actor|GetAllActorsOfClass "/Game/MyContent/Blueprints/IA/BP_ShooterCharacter.BP_ShooterCharacter_C"))
      (bind _outactors_2 (Actor|GetAllActorsOfClass "/Game/MyContent/Blueprints/IA/BP_Spider.BP_Spider_C"))
      (if (<= (- (+ (Utilities|Array|Length _outactors_2) (- (Utilities|Array|Length _outactors) 1)) 1) 0)
        (Class|KillEmAllGameMode|EndGame true)))))

(event EventBeginPlay
  (bind _outactors (Actor|GetAllActorsOfClass "/Game/MyContent/Blueprints/IA/BP_ShooterCharacter.BP_ShooterCharacter_C"))
  (for _array_element _outactors
    (Game|BindEventtoOnDestroyed _array_element (delegate Custom|EventDestroy)))
  (bind _outactors_2 (Actor|GetAllActorsOfClass "/Game/MyContent/Blueprints/IA/BP_Spider.BP_Spider_C"))
  (for _array_element_2 _outactors_2
    (Game|BindEventtoOnDestroyed _array_element_2 (delegate Custom|EventDestroy))))

(event EventTick
  (params (DeltaSeconds :type Float%20%28single-precision%29)))

(fn ConstructionScript)