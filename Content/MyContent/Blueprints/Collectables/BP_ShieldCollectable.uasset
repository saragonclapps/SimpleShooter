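; BP_ShieldCollectable is a pickup that adds shield to the player's ShooterCharacter.
; On overlap it stores the player character and calls the parent's overlap logic only if the shield is not full.
; At BeginPlay it binds Execute to the collected event, which calls AddShield using the HealthPickupAmount variable, despite that variable's health-related name.
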(event Custom|Execute
  (Class|ShooterCharacter|AddShield (Variables|Default|GetShooter%20Character) (Variables|Default|GetHealth%20Pickup%20Amount)))

(event EventBeginPlay
  (EventDispatchers|BindEventtoOnCollected (delegate Custom|Execute)))

(event Collision|EventActorBeginOverlap
  (params (OtherActor :type Actor%20Object%20Reference))
  (Utilities|IsPlayer OtherActor
    (:IsPlayer
      (bind _asshooter_character (Utilities|Casting|CastToShooterCharacter OtherActor))
      (Variables|Default|SetShooter%20Character _asshooter_character)
      (if (not (Class|ShooterCharacter|IsFullShield _asshooter_character))
        (|CallParentFunction (Variables|Default|GetShooter%20Character))))))

(event EventTick
  (params (DeltaSeconds :type Float%20%28single-precision%29))
  (|CallParentFunction DeltaSeconds) ; This node is disabled and will not be called.\nDrag off pins to build functionality.
)

(fn ConstructionScript
  (|CallParentFunction))