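; Base collectable pickup actor that spins every tick and is collected when the player overlaps it.
; On overlap it stores its start values, then one timeline pulls it toward the player's current location, shrinks it to zero and drives its point light intensity.
; The light takes the curve value directly, leaving the stored starting intensity unused.
; When the timeline finishes, it calls the OnCollected dispatcher and destroys itself.
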(event Custom|Event%20Collected
  (Actor|DestroyActor))

(event EventTick
  (params (DeltaSeconds :type Float%20%28single-precision%29))
  (Transformation|AddActorLocalRotation "0,2.000000, 0" false false))

(event Collision|EventActorBeginOverlap
  (params (OtherActor :type Actor%20Object%20Reference))
  (Utilities|IsPlayer OtherActor
    (:IsPlayer
      (CallFunction|StoreStartingValues)
      (bind (_direction _alpha_actor_location _alpha_actor_scale _alpha_light_intensity) (Timeline|Collection%20Timeline Play)
        (:Update
          (CallFunction|MovetoPlayer _alpha_actor_location)
          (CallFunction|ObjectScaleto0 _alpha_actor_scale)
          (CallFunction|ChangesIntensity0 _alpha_light_intensity))
        (:Finished
          (Default|CallOnCollected)
          (Actor|DestroyActor))))))

(fn ConstructionScript)

(fn StoreStartingValues
  (Variables|Default|SetStart%20Location (Transformation|GetActorLocation))
  (Variables|Default|SetStart%20Scale (Transformation|GetActorScale3D))
  (Variables|Default|SetStart%20Light%20Intensity (Variables|/Script/Engine.LightComponentBase|GetIntensity (Variables|Default|GetPointLight))))

(fn MovetoPlayer
  (params (Alpha :type Float%20%28single-precision%29))
  (Transformation|SetActorLocation (Math|Vector|Lerp(Vector) (Variables|Default|GetStart%20Location) (Transformation|GetActorLocation (Game|GetPlayerCharacter 0)) Alpha) false false))

(fn ObjectScaleto0
  (params (Alpha :type Float%20%28single-precision%29))
  (Transformation|SetActorScale3D (Math|Vector|Lerp(Vector) (Variables|Default|GetStart%20Scale) "0, 0, 0" Alpha)))

(fn ChangesIntensity0
  (params (NewParam :type Float%20%28single-precision%29))
  (Rendering|Components|Light|SetIntensity (Variables|Default|GetPointLight) NewParam))