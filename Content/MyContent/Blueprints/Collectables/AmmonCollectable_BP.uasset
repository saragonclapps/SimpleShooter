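; Ammo pickup collectable that refills the player's current gun when collected.
; On overlap it confirms the actor is the player, caches the shooter character, and passes to the parent overlap logic only if ammo is not full.
; An Execute handler bound to OnCollected at BeginPlay adds ammo to the current gun, reusing the HealthPickupAmount variable as the amount.
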(event Custom|Execute
  (bind _returnvalue (Class|ShooterCharacter|GetCurrentGun (Variables|Default|GetShooter%20Character)))
  (Class|Gun|AddAmmon _returnvalue (Variables|Default|GetHealth%20Pickup%20Amount)))

(event EventBeginPlay
  (EventDispatchers|BindEventtoOnCollected (delegate Custom|Execute)))

(event Collision|EventActorBeginOverlap
  (params (OtherActor :type Actor%20Object%20Reference))
  (Utilities|IsPlayer OtherActor
    (:IsPlayer
      (bind _asshooter_character (Utilities|Casting|CastToShooterCharacter OtherActor))
      (Variables|Default|SetShooter%20Character _asshooter_character)
      (if (not (Class|ShooterCharacter|IsAmmonFull _asshooter_character))
        (|CallParentFunction (Variables|Default|GetShooter%20Character))))))

(event EventTick
  (params (DeltaSeconds :type Float%20%28single-precision%29))
  (|CallParentFunction DeltaSeconds) ; This node is disabled and will not be called.\nDrag off pins to build functionality.
)

(fn ConstructionScript
  (|CallParentFunction))